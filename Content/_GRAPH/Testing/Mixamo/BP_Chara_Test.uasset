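; BP_Chara_Test is a test actor that previews an ash dissolve effect on a dancing Mixamo character mesh.
; Holding debug key G activates the Niagara ash effect and, after a one-second delay, plays a timeline driving the mesh materials' Full_Black and Dissolve parameters.
; Releasing G deactivates the particles and reverses the timeline.
; BeginPlay enables input for player 0; leftover Full_Black reset and Propagation nodes never run.
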(event EventBeginPlay
  (Input|EnableInput (Game|GetPlayerController 0)))

(event Collision|EventActorBeginOverlap
  (params (OtherActor :type Actor%20Object%20Reference)))

(event EventTick
  (params (DeltaSeconds :type Float%20%28single-precision%29)))

(event Input|KeyboardEvents|DebugKeyG
  (params (Key :type Key%20Structure :default "None") (ActionValue :type Input%20Action%20Value%20Structure))
  (bind _ns_ashes_blowaway (Variables|Default|GetNS_Ashes_Blowaway))
  (:Pressed
    (Components|Activation|SetActive _ns_ashes_blowaway true false)
    (Utilities|FlowControl|Delay 1.0)
    (bind (_direction _dissolve_time _0_to_1_curved _0_to_1_straight) (Timeline|Timeline1 Play)
      (:Update
        (Rendering|Material|SetScalarParameterValueonMaterials (Variables|Default|GetDancing_Twerk) "Full_Black" _0_to_1_curved)
        (Rendering|Material|SetScalarParameterValueonMaterials (Variables|Default|GetDancing_Twerk) "Dissolve" _dissolve_time))))
  (:Released
    (Components|Activation|SetActive _ns_ashes_blowaway false false)
    (Timeline|Timeline1 Reverse)))

(fn ConstructionScript)